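; BP_OverlapBox is a one-shot trigger cube in the shooting game that spawns a BP_Weapon when something overlaps it.
; The overlap is handled only with authority, which hides the cube, disables its collision and spawns the weapon at the box's transform.
; It then calls ResBeginOverlap, a custom event that repeats the hide and collision shutoff on the cube.
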(event OnComponentBeginOverlap(Cube)
  (params (OverlappedComponent :type Primitive%20Component%20Object%20Reference) (OtherActor :type Actor%20Object%20Reference) (OtherComp :type Primitive%20Component%20Object%20Reference) (OtherBodyIndex :type Integer) (bFromSweep :type Boolean) (SweepResult :type Hit%20Result%20Structure%20%28by%20ref%29))
  (bind _cube (Variables|Default|GetCube))
  (Networking|SwitchHasAuthority
    (:Authority
      (Rendering|SetVisibility _cube false false)
      (Collision|SetCollisionEnabled _cube "NoCollision")
      (Game|SpawnActorfromClass "/Game/ShootingGame/Blueprints/BP_Weapon.BP_Weapon_C" (Transformation|GetActorTransform) "Undefined" 0 0)
      (CallFunction|ResBeginOverlap))))

(event Custom|ResBeginOverlap
  (bind _cube (Variables|Default|GetCube))
  (Rendering|SetVisibility _cube false false)
  (Collision|SetCollisionEnabled _cube "NoCollision"))

(fn ConstructionScript)