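; Burst-fire weapon Blueprint for the shooting game that plays three rifle shots per trigger pull.
; PullTrigger plays the single-shot montage on the passed character, sets a counter and starts a looping timer.
; AdditionalShoot replays the montage on OwnCharacter until the counter runs out, then clears the timer.
; ReleaseTrigger is empty, and this Blueprint contains no projectile or damage logic, only montage playback.
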(event EventBeginPlay)

(event Collision|EventActorBeginOverlap
  (params (OtherActor :type Actor%20Object%20Reference)))

(event EventTick
  (params (DeltaSeconds :type Float%20%28single-precision%29)))

(fn ConstructionScript
  (|CallParentFunction))

(fn PullTrigger
  (params (Character :type Character%20Object%20Reference))
  (Animation|PlayAnimMontage Character "/Game/RifleAnimsetPro/Animations/InPlace/Rifle_ShootOnce_Montage.Rifle_ShootOnce_Montage" 1.0 "None")
  (Variables|Default|SetFireCount 2)
  (Utilities|Time|SetTimerbyFunctionName 0 "AdditionalShoot" 0.1 true))

(fn ReleaseTrigger)

(fn AdditionalShoot
  (bind _owncharacter (Variables|Default|GetOwnCharacter))
  (Utilities|IsValid _owncharacter
    (:Is%20Valid
      (if (> (Variables|Default|GetFireCount) 0)
        (Animation|PlayAnimMontage _owncharacter "/Game/RifleAnimsetPro/Animations/InPlace/Rifle_ShootOnce_Montage.Rifle_ShootOnce_Montage" 1.0 "None")
        (Math|Integer|DecrementInt (Variables|Default|GetFireCount))
        (else
          (Utilities|Time|ClearTimerbyFunctionName 0 "AdditionalShoot"))))))