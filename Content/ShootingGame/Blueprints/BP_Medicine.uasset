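; BP_Medicine is a healing item for the shooting game that restores health to the character using it.
; UseItem runs the parent check first, then adds a fixed heal through the character's BP_ShootingPlayerState and destroys the actor.
; HideMedicine and ShowMedicine toggle the static mesh's visibility and collision together.
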(fn ConstructionScript)

(fn HideMedicine
  (bind _staticmesh (Variables|Default|GetStaticMesh))
  (Rendering|SetVisibility _staticmesh false false)
  (Collision|SetCollisionEnabled _staticmesh "NoCollision"))

(fn ShowMedicine
  (bind _staticmesh (Variables|Default|GetStaticMesh))
  (Rendering|SetVisibility _staticmesh true false)
  (Collision|SetCollisionEnabled _staticmesh "QueryAndPhysics"))

(fn UseItem
  (params (Character :type Character%20Object%20Reference))
  (bind _isuse (|CallParentFunction Character))
  (if _isuse
    (bind _asbp_shooting_player_state (Utilities|Casting|CastToBP_ShootingPlayerState (Variables|/Script/Engine.Pawn|GetPlayerState Character)))
    (Default|AddHeal _asbp_shooting_player_state 5e+01)
    (Actor|DestroyActor)))