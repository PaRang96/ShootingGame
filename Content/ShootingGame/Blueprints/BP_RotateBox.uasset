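; BP_RotateBox is an interactable box actor in the shooting game whose Cube mesh can be set spinning.
; A press event calls EnablePlay, which toggles IsPlaying, while the release event does nothing; both return false.
; While IsPlaying is set, Tick adds a fixed relative rotation to the Cube each frame, so spin speed depends on frame rate.
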(event EventTick
  (params (DeltaSeconds :type Float%20%28single-precision%29))
  (if (Variables|Default|GetIsPlaying)
    (Transformation|AddRelativeRotation (Variables|Default|GetCube) "0,10.000000,0.000000" false false)))

(fn ConstructionScript)

(fn EnablePlay
  (Variables|Default|SetIsPlaying (not (Variables|Default|GetIsPlaying))))

(fn EventPressed
  (params (Character :type Character%20Object%20Reference))
  (CallFunction|EnablePlay)
  (return false))

(fn EventReleased
  (params (Character :type Character%20Object%20Reference))
  (return false))