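; BP_ArmourPlate is a usable item in the shooting game that grants armour to the character using it.
; It overrides UseItem and continues only if the parent implementation returns true.
; It then casts the character's PlayerState to BP_ShootingPlayerState, adds a fixed amount of armour there and destroys itself.
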(event EventBeginPlay
  (|CallParentFunction) ; This node is disabled and will not be called.\nDrag off pins to build functionality.
)

(event EventTick
  (params (DeltaSeconds :type Float%20%28single-precision%29))
  (|CallParentFunction DeltaSeconds) ; This node is disabled and will not be called.\nDrag off pins to build functionality.
)

(fn ConstructionScript
  (|CallParentFunction))

(fn UseItem
  (params (Character :type Character%20Object%20Reference))
  (bind _isuse (|CallParentFunction Character))
  (if _isuse
    (bind _asbp_shooting_player_state (Utilities|Casting|CastToBP_ShootingPlayerState (Variables|/Script/Engine.Pawn|GetPlayerState Character)))
    (Default|AddArmour _asbp_shooting_player_state 5e+01)
    (Actor|DestroyActor)))