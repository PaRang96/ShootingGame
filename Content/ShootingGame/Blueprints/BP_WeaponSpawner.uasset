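; BP_WeaponSpawner spawns weapon actors from the T_WeaponTable data table at its own transform when play begins, on the server only.
; If the configured WeaponName is a valid row, it spawns SpawnCount copies of that weapon.
; Otherwise, it picks a random row for each spawn.
; Each actor uses the row's WeaponClass and receives the row data as WeaponRef.
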(event EventBeginPlay
  (bind _weaponname (Variables|Default|GetWeaponName))
  (Networking|SwitchHasAuthority
    (:Authority
      (bind _returnvalue (Class|DataTableFunctionLibrary|DoesDataTableRowExist "/Game/ShootingGame/Data/T_WeaponTable.T_WeaponTable" _weaponname))
      (if _returnvalue
        (for _index (range 1 (Variables|Default|GetSpawnCount))
          (CallFunction|SpawnActorbyName _weaponname))
        (else
          (for _index_2 (range 1 (Variables|Default|GetSpawnCount))
            (CallFunction|SpawnActorbyName (CallFunction|GetRandomWeaponName))))))))

(fn ConstructionScript)

(fn SpawnActorbyName
  (params (RowName :type Name))
  (bind _returnvalue (Utilities|GetDataTableRow "/Game/ShootingGame/Data/T_WeaponTable.T_WeaponTable" RowName)
    (:then
      (Game|SpawnActorfromClass (.WeaponClass (Utilities|Struct|BreakST_Weapon _returnvalue)) (Transformation|GetActorTransform) "Undefined" 0 _returnvalue 0))))

(fn GetRandomWeaponName
  (bind _outrownames (DataTable|GetDataTableRowNames "/Game/ShootingGame/Data/T_WeaponTable.T_WeaponTable"))
  (return (Utilities|Array|Get(acopy) _outrownames (Math|Random|RandomInteger (Utilities|Array|Length _outrownames)))))