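; BP_Magazine is a spinning magazine pickup for the shooting game that adds one to a character's Mag count when used.
; UseItem runs the parent check, stores the shooting character, increments its Mag, then destroys the pickup.
; The HUD magazine count updates only when that character is controlled by player controller 0.
; Show and hide functions toggle the mesh's visibility and collision together, while Tick drives the yaw spin.
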(event EventTick
  (params (DeltaSeconds :type Float%20%28single-precision%29))
  (Transformation|AddRelativeRotation (Variables|Default|GetStaticMesh) (Math|Rotator|MakeRotator 0.0 0.0 (* 150 (+ DeltaSeconds (Variables|Default|GetTime)))) false false))

(fn ConstructionScript)

(fn UpdateUIMag
  (params (Value :type Integer))
  (Utilities|CheckMyPlayer
    (:True
      (bind _asbp_shooting_hud (Utilities|Casting|CastToBP_ShootingHUD (HUD|GetHUD (Game|GetPlayerController 0))))
      (Default|UpdateMag _asbp_shooting_hud Value))))

(fn AddMag
  (params (BPShootingCharacter :type BP%20Shooting%20Character%20Object%20Reference))
  (bind _output_get (Variables|/Game/ShootingGame/GameMode/BP_ShootingCharacter.BP_ShootingCharacter_C|SetMag BPShootingCharacter (+ (Variables|/Game/ShootingGame/GameMode/BP_ShootingCharacter.BP_ShootingCharacter_C|GetMag BPShootingCharacter) 1)))
  (CallFunction|UpdateUIMag _output_get))

(fn HideMagazine
  (bind _staticmesh (Variables|Default|GetStaticMesh))
  (Collision|SetCollisionEnabled _staticmesh "NoCollision")
  (Rendering|SetVisibility _staticmesh false false))

(fn ShowMagazine
  (bind _staticmesh (Variables|Default|GetStaticMesh))
  (Collision|SetCollisionEnabled _staticmesh "QueryAndPhysics")
  (Rendering|SetVisibility _staticmesh true false))

(fn UseItem
  (params (Character :type Character%20Object%20Reference))
  (bind _isuse (|CallParentFunction Character))
  (if _isuse
    (bind _asbp_shooting_character (Utilities|Casting|CastToBP_ShootingCharacter Character))
    (bind _output_get (Variables|Default|SetOwnCharacter _asbp_shooting_character))
    (CallFunction|AddMag _output_get)
    (Actor|DestroyActor)))