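; Lobby player state that holds a player's Name and announces changes to it.
; On BeginPlay it passes itself to the first player controller's BP_LobbyHUD for binding, printing an error if the cast fails.
; SetName writes the Name variable, whose RepNotify prints the value and fires the ChangeName dispatcher with it.
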(event EventBeginPlay
  (CallFunction|InitBind))

(fn ConstructionScript)

(fn OnRepName
  (Development|PrintString (Utilities|String|Append "On Rep Name: " (Variables|Default|GetName)) true true "(R=0.000000,G=0.660000,B=1.000000,A=1.000000)" 6e+01)
  (Default|CallChangeNameDispatcher (Variables|Default|GetName)))

(fn SetName
  (params (Name :type String))
  (Variables|Default|SetName Name))

(fn InitBind
  (bind _asbp_lobby_hud (Utilities|Casting|CastToBP_LobbyHUD (HUD|GetHUD (Game|GetPlayerController 0)))
    (:then
      (Default|BindPlayerState _asbp_lobby_hud self))
    (:CastFailed
      (Development|PrintString "BP_Lobby HUD Cast Fail" true true "(R=1.000000,G=0.000000,B=0.000000,A=1.000000)" 6e+01))))