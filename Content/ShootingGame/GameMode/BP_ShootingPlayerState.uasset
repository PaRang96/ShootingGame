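; Player state for the shooting game that holds a player's replicated HP and armour, with functions for damage, healing, armour pickup and revive.
; Damage drains armour first; a hit that armour cannot cover zeroes it, then subtracts the full damage from HP, as armour is cleared before the subtraction.
; RepNotify functions broadcast both values through dispatchers, leaving older direct name tag and HUD update code disconnected.
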(event EventBeginPlay
  (Development|PrintString (Utilities|String|Append "create: " (Utilities|GetDisplayName self) " Pawn:" (Utilities|GetDisplayName (Variables|Default|GetPawnPrivate))) true true "(R=0.000000,G=0.660000,B=1.000000,A=1.000000)" 6e+01))

(fn ConstructionScript)

(fn AddDamage
  (params (Damage :type Float%20%28single-precision%29))
  (if (> (- (Variables|Default|GetArmour) Damage) 0.0)
    (Variables|Default|SetArmour (- (Variables|Default|GetArmour) Damage))
    (else
      (Variables|Default|SetArmour 0.0)
      (bind _output_get (Variables|Default|SetHP (Math|Float|Clamp(Float) (+ (Variables|Default|GetHP) (- (Variables|Default|GetArmour) Damage)) 0.0 1e+02)))
      (Development|PrintString (Utilities|String|ToString(Float) _output_get)))))

(fn OnRepHP
  (Default|CallHPDispatcher (Variables|Default|GetHP) 1e+02))

(fn Revive
  (Variables|Default|SetHP 1e+02))

(fn AddHeal
  (params (Heal :type Float%20%28single-precision%29))
  (Variables|Default|SetHP (Math|Float|Clamp(Float) (+ (Variables|Default|GetHP) Heal) 0.0 1e+02)))

(fn OnRepArmour
  (Default|CallArmourDispatcher (Variables|Default|GetArmour) 1e+02))

(fn AddArmour
  (params (Armour :type Float%20%28single-precision%29))
  (Variables|Default|SetArmour (Math|Float|Clamp(Float) (+ (Variables|Default|GetArmour) Armour) 0.0 1e+02)))